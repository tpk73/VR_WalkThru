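; BP_Light is a VR interactible tower light that toggles on and off when its Activate event is called.
; A FlipFlop alternates six spotlights between zero and full working intensity, switching them off on the first call.
; Both branches assign the same tower light material to the Light component, so only the spotlight intensity differs between states.
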(event EventBeginPlay)

(event Collision|EventActorBeginOverlap
  (params (OtherActor :type Actor%20Object%20Reference)))

(event EventTick
  (params (DeltaSeconds :type Float%20%28single-precision%29)))

(event EventActivate
  (Utilities|FlowControl|FlipFlop
    (:A
      (Rendering|Components|Light|SetIntensity (Variables|Default|GetSpotLight) 0.0)
      (Rendering|Material|SetMaterial (Variables|Default|GetLight) 0 "/Game/Military_Assets/Locations/MilitaryBase/Materials/MI_TowerLight01.MI_TowerLight01"))
    (:B
      (Rendering|Components|Light|SetIntensity (Variables|Default|GetSpotLight) 8.0)
      (Rendering|Material|SetMaterial (Variables|Default|GetLight) 0 "/Game/Military_Assets/Locations/MilitaryBase/Materials/MI_TowerLight01.MI_TowerLight01"))))

(fn ConstructionScript)